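; General enemy character that performs melee attacks, takes damage and dies, with a health bar widget refreshed every tick.
; AttackPlayer plays a random attack montage; AoeBox overlaps during it deal fixed damage, throttled by a DoOnce that resets after a delay.
; Incoming damage, except its own, reduces Health, spawns screen-projected floating combat text and prints health.
; It then plays a hit reaction, or a death montage that disables movement and destroys the actor.
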(event OnComponentBeginOverlap(AoeBox)
  (params (OverlappedComponent :type Primitive%20Component%20Object%20Reference) (OtherActor :type Actor%20Object%20Reference) (OtherComp :type Primitive%20Component%20Object%20Reference) (OtherBodyIndex :type Integer) (bFromSweep :type Boolean) (SweepResult :type Hit%20Result%20Structure%20%28by%20ref%29))
  (bind _returnvalue (Pawn|GetController))
  (if (Variables|Default|GetIsAttacking)
    (Utilities|FlowControl|DoOnce false :!label _label
      (:Completed
        (Game|Damage|ApplyDamage OtherActor 2e+01 _returnvalue _returnvalue)
        (Utilities|FlowControl|Delay 1.0)
        (goto _label Reset)))))

(event Custom|AttackPlayer
  (bind _attackmontage (Variables|Default|GetAttackMontage))
  ;[1 1 1] Attack
  (if (not (Variables|Default|GetisDying))
    (if (not (Variables|Default|GetIsAttacking))
      (Variables|Default|SetIsAttacking true)
      (Animation|Montage|PlayMontage (Variables|Character|GetMesh) (Utilities|Array|Get(acopy) _attackmontage (Math|Random|RandomInteger (Utilities|Array|Length _attackmontage)))
        (:OnCompleted
          _)
        (:OnBlendOut
          _)
        (:OnInterrupted
          _))
      (Variables|Default|SetIsAttacking false))))

(event Game|Damage|EventAnyDamage
  (params (Damage :type Float%20%28single-precision%29) (DamageType :type Damage%20Type%20Object%20Reference) (InstigatedBy :type Controller%20Object%20Reference) (DamageCauser :type Actor%20Object%20Reference))
  (if (!= InstigatedBy (Pawn|GetController))
    (if (not (Variables|Default|GetisDying))
      (bind _output_get (Variables|Default|SetHealth (- (Variables|Default|GetHealth) Damage)))
      (CallFunction|SpawnFloatingCombatText (Transformation|GetActorLocation) Damage)
      (Development|PrintString (Utilities|String|ToString(Float) _output_get))
      (if (<= _output_get 0.0)
        (Animation|Montage|PlayMontage (Variables|Character|GetMesh) "/Game/Enemy/Zombie/Montage/Zombie_Dying2_Montage.Zombie_Dying2_Montage"
          (:then
            (Variables|Default|SetisDying true)
            (Pawn|Components|CharacterMovement|DisableMovement (Variables|Character|GetCharacterMovement)))
          (:OnCompleted
            (Actor|DestroyActor :!label _label))
          (:OnBlendOut
            (goto _label)))
        (else
          (Animation|Montage|PlayMontage (Variables|Character|GetMesh) "/Game/Enemy/Zombie/Montage/Standing_React_Large_From_Left_Montage.Standing_React_Large_From_Left_Montage"
            (:then
              (Utilities|FlowControl|Delay 1.0))))))))

(event EventTick
  (params (DeltaSeconds :type Float%20%28single-precision%29))
  (bind _asblood_bp_2 (Utilities|Casting|CastToBlood_BP_2 (UserInterface|GetWidget (Variables|Default|GetBlood))))
  (Default|SetGeneralBloodPercentage _asblood_bp_2 self))

(fn ConstructionScript)

(fn SpawnFloatingCombatText
  (params (WorldPosition :type Vector%20%28by%20ref%29) (DamageToDisplay :type Float%20%28single-precision%29))
  (bind _returnvalue (UserInterface|CreateWidget "/Game/UI/FloatingText.FloatingText_C" 0 DamageToDisplay (.ScreenPosition (Class|GameplayStatics|ProjectWorldtoScreen (Game|GetPlayerController 0) WorldPosition false))))
  (UserInterface|Viewport|AddtoViewport _returnvalue 0))